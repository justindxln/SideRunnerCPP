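; BP_PlayerStatusManager relays player status changes to the HUD widget so it can play the matching animations.
; DoSetHUDReference casts and caches the HUD widget reference used by every other event.
; One-shot events forward added health, damage and score boost, while toggle events pass an Active flag for speed, healing and shield effects.
; It holds no status logic itself, and the forwarding events do not check that the reference is valid.
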(event EventDoSetHUDReference
  ;[1 1 1] Play Animations in HUD Widget
  (bind _ashudwidget (Utilities|Casting|CastToHUDWidget (Variables|Default|GetHUDWidget)))
  (Variables|Default|SetAs%20HUDWidget _ashudwidget))

(event EventDoHUDToggleHealing
  (params (bActive :type Boolean))
  ;[1 1 1] Play Animations in HUD Widget
  (Default|ToggleHealStatus (Variables|Default|GetAs%20HUDWidget) bActive))

(event EventDoHUDToggleShield
  (params (bActive :type Boolean))
  ;[1 1 1] Play Animations in HUD Widget
  (Default|ToggleShield (Variables|Default|GetAs%20HUDWidget) bActive))

(event EventDoHUDToggleSpeed
  (params (bActive :type Boolean))
  ;[1 1 1] Play Animations in HUD Widget
  (Default|ToggleSpeedBuff (Variables|Default|GetAs%20HUDWidget) bActive))

(event EventDoHUDApplyScoreBoost
  ;[1 1 1] Play Animations in HUD Widget
  (Default|DoScoreBoost (Variables|Default|GetAs%20HUDWidget)))

(event EventDoHUDAddHealth
  ;[1 1 1] Play Animations in HUD Widget
  (Default|DoAddHealth (Variables|Default|GetAs%20HUDWidget)))

(event EventDoHUDTakeDamage
  ;[1 1 1] Play Animations in HUD Widget
  (Default|DoTakeDamage (Variables|Default|GetAs%20HUDWidget)))

(fn ConstructionScript)